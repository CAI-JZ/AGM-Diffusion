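; Test actor for an absorb-style disappearing effect that shrinks a static mesh alongside a Niagara particle system.
; On BeginPlay a timeline plays in reverse from its end, driving the mesh's world scale from its track.
; The same track interpolates the Niagara spawn rate and particle size parameters, so both fall off with the track value.
; An unconnected node for overriding the Niagara sample mesh with a rock never runs.
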(event `self.ReceiveBeginPlay`
  (bind _niagara (`self.Niagara`))
  ;[1 1 1] Disappear ( 我要做消失，这里是缩小）
  (bind (_direction _newtrack_0) (`Timeline|Timeline_0` :!via `ReverseFromEnd`)
    (:`Update`
      (`SceneComponent.SetWorldScale3D` (`self.StaticMesh`) (`KismetMathLibrary.Conv_DoubleToVector` _newtrack_0))
      (`FXSystemComponent.SetFloatParameter` _niagara "SpawnRate_New" (`KismetMathLibrary.Lerp` 0.0 (`self.B`) _newtrack_0))
      (`FXSystemComponent.SetFloatParameter` _niagara "New_Size" (`KismetMathLibrary.Lerp` 0.01 0.1 _newtrack_0)))))

(fn `UserConstructionScript`)