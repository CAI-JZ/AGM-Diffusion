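; BP_Fire is a fire obstacle actor that the player's ball can absorb or put out with water.
; Absorb and Water both call FireDisappear, which disables the blocking box's collision, destroys the particle system and shows a plane and ash smoke.
; Absorb then sets the player PB_MainBall's SkillIndex to fire and applies the Trail_Fire material, while Water calls ResetMatter on the ball.
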(event `/Game/Blueprint/BPI_MainBallSkill.Absorb`
  (`self.FireDisappear`)
  (bind _aspb_main_ball (cast `/Game/Blueprint/PB_MainBall` (`GameplayStatics.GetPlayerPawn` 0)))
  (set `/Game/Blueprint/PB_MainBall.SkillIndex` 1 _aspb_main_ball)
  (`PrimitiveComponent.SetMaterial` (`/Game/Blueprint/PB_MainBall.Sphere` _aspb_main_ball) 0 "/Game/Materials/Material/Trail_Fire.Trail_Fire")
  (`PrimitiveComponent.SetMaterial` (`/Game/Blueprint/PB_MainBall.PlaneSkill` _aspb_main_ball) 0 "/Game/Materials/Material/Trail_Fire.Trail_Fire"))

(event `/Game/Blueprint/BPI_MainBallSkill.Water`
  (`self.FireDisappear`)
  (bind _aspb_main_ball (cast `/Game/Blueprint/PB_MainBall` (`GameplayStatics.GetPlayerPawn` 0)))
  (`/Game/Blueprint/PB_MainBall.ResetMatter` _aspb_main_ball))

(fn `FireDisappear`
  (`|ExecutionSequence`
    (:`then_0`
      (`PrimitiveComponent.SetCollisionEnabled` (`self.BoxBlock`) "NoCollision")
      (`ActorComponent.K2_DestroyComponent` (`self.ParticleSystem`)))
    (:`then_1`
      (`SceneComponent.SetVisibility` (`self.Plane`) true false)
      (`SceneComponent.SetVisibility` (`self.Ash&Smoke`) true false))))

(fn `UserConstructionScript`)