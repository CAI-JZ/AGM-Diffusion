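; Main ball the player steers in 100-unit steps, with elemental skills used on objects ahead.
; WASD sets facing and Space moves when a forward trace is clear and a downward trace finds ground.
; Tick highlights that ground actor, using the game instance's HighLightActor to clear the previous one.
; SkillIndex gates Absorb (normal state) or picks Fire, Water or Ice, sent to the traced actor through BPI_MainBallSkill; ResetMatter restores normal.
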(event `Key|R`
  (params (Key :type "Key Structure"))
  ;[1 1 1] Test
)

(event `Key|One`
  (params (Key :type "Key Structure"))
  ;[1 1 1] Test
)

(event `InputAction|UseFeature`
  (params (Key :type "Key Structure"))
  ;[1 1 1] Skill
  (:`Released`
    (bind _ishit (`self.TraceForward`))
    (if _ishit
      (switch `int` (`self.SkillIndex`)
        (:`1`
          (`self.FireSkill`))
        (:`2`
          (`self.WaterSkill`))
        (:`3`
          (`self.IceSkill`))))))

(event `InputAction|AbsorbElement`
  (params (Key :type "Key Structure"))
  (bind _itemre (`self.ItemRe`))
  ;[1 1 1] Absorb Element
  (:`Released`
    (bind _ishit (`self.TraceForward`))
    (if _ishit
      (if (== (`self.SkillIndex`) 0)
        (if (`KismetSystemLibrary.DoesImplementInterface` _itemre "/Game/Blueprint/BPI_MainBallSkill.BPI_MainBallSkill_C")
          (message `/Game/Blueprint/BPI_MainBallSkill.Absorb` _itemre))))))

(event `ResetMatter`
  ;[1 1 1] Change to Normal
  (set `self.SkillIndex` 0)
  (`PrimitiveComponent.SetMaterial` (`self.Sphere`) 0 "/Game/Materials/Material/Trail_Test.Trail_Test"))

(event `FireSkill`
  (bind _itemre (`self.ItemRe`))
  ;[1 1 1] FireSkill
  (if (`self.IsOverlap_MainChar`)
    (if (`KismetSystemLibrary.DoesImplementInterface` _itemre "/Game/Blueprint/BPI_MainBallSkill.BPI_MainBallSkill_C")
      (message `/Game/Blueprint/BPI_MainBallSkill.Fire` _itemre))))

(event `WaterSkill`
  (bind _itemre (`self.ItemRe`))
  ;[1 1 1] WaterSkill
  (if (`self.IsOverlap_MainChar`)
    (if (`KismetSystemLibrary.DoesImplementInterface` _itemre "/Game/Blueprint/BPI_MainBallSkill.BPI_MainBallSkill_C")
      (message `/Game/Blueprint/BPI_MainBallSkill.Water` _itemre))))

(event `IceSkill`
  (bind _itemre (`self.ItemRe`))
  ;[1 1 1] Ice Skill
  (if (`self.IsOverlap_MainChar`)
    (if (`KismetSystemLibrary.DoesImplementInterface` _itemre "/Game/Blueprint/BPI_MainBallSkill.BPI_MainBallSkill_C")
      (message `/Game/Blueprint/BPI_MainBallSkill.Ice` _itemre))))

(event `self.ReceiveTick`
  (params (DeltaSeconds :type "Float (single-precision)"))
  ;[1 1 1] Highlight Trace Square
  (bind (_istouch _forworditem) (`self.TraceDown`))
  (set `self.Is Touch` _istouch)
  (set `self.ForwordItem` _forworditem)
  (bind _asbp_instance (cast `/Game/Blueprint/BP_Instance` (`GameplayStatics.GetGameInstance`)))
  (bind _highlightactor (`/Game/Blueprint/BP_Instance.HighLightActor` _asbp_instance))
  (`/Engine/EditorBlueprintResources/StandardMacros.IsValid` _highlightactor
    (:`Is Valid`
      (if (`self.Is Touch`)
        (if (== _highlightactor (`self.ForwordItem`))
          (message `/Game/Blueprint/BPI_MainBallSkill.Hightlight` (`self.ForwordItem`))
          (else
            (message `/Game/Blueprint/BPI_MainBallSkill.StopHighLight` _highlightactor)
            (`KismetSystemLibrary.Delay` 0.01)
            (message `/Game/Blueprint/BPI_MainBallSkill.Hightlight` (`self.ForwordItem`))))
        (else
          (message `/Game/Blueprint/BPI_MainBallSkill.StopHighLight` _highlightactor))))
    (:`Is Not Valid`
      (message `/Game/Blueprint/BPI_MainBallSkill.Hightlight` (`self.ForwordItem`)))))

(event `Key|SpaceBar`
  (params (Key :type "Key Structure"))
  ;[1 1 1] Move
  (:`Pressed`
    (bind _ishit (`self.TraceForward`))
    (if _ishit
      _
      (elif (`self.Is Touch`)
        (`self.K2_AddActorWorldOffset` (* (`SceneComponent.GetForwardVector` (`self.Root`)) 100.0))))))

(event `Key|W`
  (params (Key :type "Key Structure"))
  ;[1 1 1] Choose direction
  (:`Pressed`
    (`SceneComponent.K2_SetRelativeRotation` (`self.Root`) (struct :`Yaw` -90.0) false false)))

(event `Key|S`
  (params (Key :type "Key Structure"))
  ;[1 1 1] Choose direction
  (:`Pressed`
    (`SceneComponent.K2_SetRelativeRotation` (`self.Root`) (struct :`Yaw` 90.0) false false)))

(event `Key|D`
  (params (Key :type "Key Structure"))
  ;[1 1 1] Choose direction
  (:`Pressed`
    (`SceneComponent.K2_SetRelativeRotation` :`self` (`self.Root`))))

(event `Key|A`
  (params (Key :type "Key Structure"))
  ;[1 1 1] Choose direction
  (:`Pressed`
    (`SceneComponent.K2_SetRelativeRotation` (`self.Root`) (struct :`Yaw` 180.0) false false)))

(fn `CheckIsOverlap`
  (params (OverlapCheck :type Boolean :default false))
  (return))

(fn `TraceDown`
  (returns (IsTouch :type Boolean) (ForwordItem :type "Actor Object Reference"))
  (locals (IsHit :type Boolean))
  (bind _returnvalue (+ (* (`SceneComponent.GetForwardVector` (`self.Arrow`)) 100.0) (`self.K2_GetActorLocation` (`GameplayStatics.GetPlayerPawn` 0))))
  (bind _outhit (`KismetSystemLibrary.LineTraceSingle` :`Start` _returnvalue :`End` (+ _returnvalue (0.0 0.0 -90.0)) :`TraceChannel` "TraceTypeQuery1" :`TraceColor` (struct :`R` 1.0 :`G` 0.175134 :`A` 1.0) :`DrawTime` 50.0))
  (bind (_bblockinghit _binitialoverlap _time _distance _location _impactpoint _normal _impactnormal _physmat _hitactor) (`GameplayStatics.BreakHitResult` _outhit))
  (bind _output_get (set `local.IsHit` _bblockinghit))
  (bind _output_get_2 (set `self.ForwordItem` _hitactor))
  (return _output_get _output_get_2))

(fn `TraceForward`
  (returns (IsHit :type Boolean))
  (bind _returnvalue (`self.K2_GetActorLocation` (`GameplayStatics.GetPlayerPawn` 0)))
  (bind _outhit (`KismetSystemLibrary.LineTraceSingle` :`Start` _returnvalue :`End` (+ (* (`SceneComponent.GetForwardVector` (`self.Arrow`)) 100.0) _returnvalue) :`TraceChannel` "TraceTypeQuery1" :`DrawTime` 50.0))
  (bind (_bblockinghit _binitialoverlap _time _distance _location _impactpoint _normal _impactnormal _physmat _hitactor) (`GameplayStatics.BreakHitResult` _outhit))
  (bind _output_get (set `self.IsOverlap_MainChar` _bblockinghit))
  (set `self.ItemRe` _hitactor)
  (return _output_get))

(fn `UserConstructionScript`)