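; BP_SquareBasicAborb is a square rock object the player can absorb to gain skill index 4.
; Absorbing plays a timeline in reverse to shrink the mesh and fade Niagara spawn rate and size, then destroys the mesh and switches PB_MainBall's skill, Niagara visibility and material.
; Highlight swaps the material and registers the actor in BP_Instance, and StopHighLight restores the material.
; Water, Ice and Fire events only play a pop sound.
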(event `/Game/Blueprint/BPI_MainBallSkill.AbsorbProcess`
  ;[1 1 1] Absorb
  (bind (_direction _newtrack_0) (`Timeline|Timeline_1` :!via `ReverseFromEnd`)
    (:`Update`
      (`SceneComponent.SetWorldScale3D` (`self.Base`) (`KismetMathLibrary.VLerp` (0.0 0.0 0.0) (1.0 1.0 1.0) _newtrack_0))
      (`self.AbsorbNiagaraSet` (`self.Niagara`) _newtrack_0))
    (:`Finished`
      (`self.RockDisappear`)
      (bind _aspb_main_ball (cast `/Game/Blueprint/PB_MainBall` (`GameplayStatics.GetPlayerPawn` 0)))
      (set `/Game/Blueprint/PB_MainBall.SkillIndex` 4 _aspb_main_ball)
      (`SceneComponent.SetVisibility` (`/Game/Blueprint/PB_MainBall.Niagara` _aspb_main_ball) true false)
      (`PrimitiveComponent.SetMaterial` (`/Game/Blueprint/PB_MainBall.Sphere` _aspb_main_ball) 0 "/Game/Materials/M_AbsorbRock.M_AbsorbRock")
      (`KismetSystemLibrary.Delay` 0.2)
      (`self.AbsorbNiagaraSet` (`self.Niagara`)))))

(event `/Game/Blueprint/BPI_MainBallSkill.Water`
  (`GameplayStatics.PlaySound2D` "/Game/One_Hundred_Game_SFX/Cues/CUE_UI_Game_Pop_3_Cue.CUE_UI_Game_Pop_3_Cue" 1.0 1.0 0.0 null null))

(event `/Game/Blueprint/BPI_MainBallSkill.Hightlight`
  ;[1 1 1] HighLight
  (`PrimitiveComponent.SetMaterial` (`self.Base`) 0 "/Game/Materials/M_Highlight_Inst_Rock.M_Highlight_Inst_Rock")
  (bind _asbp_instance (cast `/Game/Blueprint/BP_Instance` (`GameplayStatics.GetGameInstance`)))
  (set `/Game/Blueprint/BP_Instance.HighLightActor` self _asbp_instance))

(event `/Game/Blueprint/BPI_MainBallSkill.Ice`
  (`GameplayStatics.PlaySound2D` "/Game/One_Hundred_Game_SFX/Cues/CUE_UI_Game_Pop_3_Cue.CUE_UI_Game_Pop_3_Cue" 1.0 1.0 0.0 null null))

(event `/Game/Blueprint/BPI_MainBallSkill.Fire`
  (`GameplayStatics.PlaySound2D` "/Game/One_Hundred_Game_SFX/Cues/CUE_UI_Game_Pop_3_Cue.CUE_UI_Game_Pop_3_Cue" 1.0 1.0 0.0 null null))

(event `/Game/Blueprint/BPI_MainBallSkill.StopHighLight`
  (bind _base (`self.Base`))
  ;[1 1 1] StopHighLigh
  (`/Engine/EditorBlueprintResources/StandardMacros.IsValid` _base
    (:`Is Valid`
      (`PrimitiveComponent.SetMaterial` _base 0 "/Game/StylizedRuinsProps/Materials/MI_ArcBuilding01.MI_ArcBuilding01"))))

(fn `RockDisappear`
  (`ActorComponent.K2_DestroyComponent` (`self.Base`))
  (`GameplayStatics.PlaySound2D` "/Game/One_Hundred_Game_SFX/Cues/CUE_UI_Bright_Confirmation_Button_1_Cue.CUE_UI_Bright_Confirmation_Button_1_Cue" 1.0 1.0 0.0 null null))

(fn `UserConstructionScript`)