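; BP_SquareBasicType2 is a board square Blueprint that gives sound feedback for element events and can be highlighted.
; Water, Ice and Fire events each play the same pop sound cue, while AbsorbProcess plays a pop sound after a short delay.
; Hightlight swaps the Base mesh to a highlight material and registers the square as HighLightActor on the BP_Instance game instance.
; StopHighLight restores the stone material.
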(event `/Game/Blueprint/BPI_MainBallSkill.AbsorbProcess`
  (`KismetSystemLibrary.Delay` 1.2)
  (`GameplayStatics.PlaySound2D` "/Game/One_Hundred_Game_SFX/Wavs/WAV_UI_Game_Pop_3.WAV_UI_Game_Pop_3" 1.0 1.0 0.0 null null))

(event `/Game/Blueprint/BPI_MainBallSkill.Water`
  (`GameplayStatics.PlaySound2D` "/Game/One_Hundred_Game_SFX/Cues/CUE_UI_Game_Pop_3_Cue.CUE_UI_Game_Pop_3_Cue" 1.0 1.0 0.0 null null))

(event `/Game/Blueprint/BPI_MainBallSkill.Ice`
  (`GameplayStatics.PlaySound2D` "/Game/One_Hundred_Game_SFX/Cues/CUE_UI_Game_Pop_3_Cue.CUE_UI_Game_Pop_3_Cue" 1.0 1.0 0.0 null null))

(event `/Game/Blueprint/BPI_MainBallSkill.Fire`
  (`GameplayStatics.PlaySound2D` "/Game/One_Hundred_Game_SFX/Cues/CUE_UI_Game_Pop_3_Cue.CUE_UI_Game_Pop_3_Cue" 1.0 1.0 0.0 null null))

(event `/Game/Blueprint/BPI_MainBallSkill.Hightlight`
  (`PrimitiveComponent.SetMaterial` (`self.Base`) 0 "/Game/Materials/M_Highlight_Inst_Normal.M_Highlight_Inst_Normal")
  (bind _asbp_instance (cast `/Game/Blueprint/BP_Instance` (`GameplayStatics.GetGameInstance`)))
  (set `/Game/Blueprint/BP_Instance.HighLightActor` self _asbp_instance))

(event `/Game/Blueprint/BPI_MainBallSkill.StopHighLight`
  (`PrimitiveComponent.SetMaterial` (`self.Base`) 0 "/Game/StylizedRuinsProps/Materials/M_Stone02.M_Stone02"))

(fn `UserConstructionScript`)