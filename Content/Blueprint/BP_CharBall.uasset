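; Player ball character that absorbs elements from objects and uses elemental skills on them.
; While absorb or skill input is held, CanMove is off and WASD can reposition a trigger box around the ball.
; On release, the overlapped actor receives a BPI_MainBallSkill message chosen by SkillIndex: absorb at zero, otherwise fire or water.
; UseIce is never called (index 3 uses water); ResetMatter and ChangeTriggerBoxTransAbsrob are empty.
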(event `Key|W`
  (params (Key :type "Key Structure"))
  (:`Pressed`
    (`SceneComponent.K2_SetRelativeRotation` (`self.Sphere`) (struct :`Yaw` 90.0) false false)))

(event `Key|S`
  (params (Key :type "Key Structure"))
  (:`Pressed`
    (`SceneComponent.K2_SetRelativeRotation` (`self.Sphere`) (struct :`Yaw` -90.0) false false)))

(event `Key|D`
  (params (Key :type "Key Structure"))
  (:`Pressed`
    (`SceneComponent.K2_SetRelativeRotation` (`self.Sphere`) (struct :`Yaw` 180.0) false false)))

(event `Key|A`
  (params (Key :type "Key Structure"))
  (:`Pressed`
    (`SceneComponent.K2_SetRelativeRotation` :`self` (`self.Sphere`))))

(event `Key|R`
  (params (Key :type "Key Structure"))
  ;[1 1 1] Test
  (:`Pressed`
    (`self.ResetMatter`)))

(event `Key|One`
  (params (Key :type "Key Structure"))
  ;[1 1 1] Test
  (:`Pressed`
    (`KismetSystemLibrary.PrintString` (`KismetStringLibrary.Conv_BoolToString` (`self.IsOverlap_MainChar`)))
    (`KismetSystemLibrary.PrintString` (`KismetStringLibrary.Conv_IntToString` (`self.SkillIndex`)) true true (struct :`R` 0.755208 :`B` 0.013354 :`A` 1.0))))

(event `InputAction|UseFeature`
  (params (Key :type "Key Structure"))
  ;[1 1 1] Skill
  (:`Pressed`
    (set `self.PressSkill` true)
    (set `self.CanMove` false)
    (`SceneComponent.SetVisibility` (`self.PlaneSkill`) true false))
  (:`Released`
    (set `self.PressSkill` false)
    (`|ExecutionSequence`
      (:`then_0`
        (if (`self.IsOverlap_MainChar`)
          (switch `int` (`self.SkillIndex`)
            (:`1`
              (`self.UseFire`))
            (:`2`
              (`self.UseWater`))
            (:`3`
              (`self.UseWater`)))))
      (:`then_1`
        (`KismetSystemLibrary.Delay` 0.01)
        (set `self.CanMove` true)
        (`self.ResetTriggerBoxTrans` (`self.Box`) (0.0 56.0 0.0))))))

(event `self.Box.OnComponentBeginOverlap`
  (params (OverlappedComponent :type "PrimitiveComponent Object Reference") (OtherActor :type "Actor Object Reference") (OtherComp :type "PrimitiveComponent Object Reference") (OtherBodyIndex :type Integer) (bFromSweep :type Boolean) (SweepResult :type "HitResult Structure (by ref)"))
  ;[1 1 1] BoxTrigger
  (set `self.ItemRe` OtherActor)
  (set `self.IsOverlap_MainChar` true))

(event `InputAction|AbsorbElement`
  (params (Key :type "Key Structure"))
  (bind _itemre (`self.ItemRe`))
  ;[1 1 1] Absorb Element
  (:`Pressed`
    (set `self.PressAbsorb` true)
    (set `self.CanMove` false)
    (`SceneComponent.SetVisibility` (`self.Plane`) true false))
  (:`Released`
    (set `self.PressAbsorb` false)
    (`|ExecutionSequence`
      (:`then_0`
        (if (`self.IsOverlap_MainChar`)
          (if (== (`self.SkillIndex`) 0)
            (if (`KismetSystemLibrary.DoesImplementInterface` _itemre "/Game/Blueprint/BPI_MainBallSkill.BPI_MainBallSkill_C")
              (message `/Game/Blueprint/BPI_MainBallSkill.Absorb` _itemre)))))
      (:`then_1`
        (set `self.CanMove` true)
        (`self.ResetTriggerBoxTrans` (`self.Box`) (0.0 56.0 0.0))))))

(event `self.Box.OnComponentEndOverlap`
  (params (OverlappedComponent :type "PrimitiveComponent Object Reference") (OtherActor :type "Actor Object Reference") (OtherComp :type "PrimitiveComponent Object Reference") (OtherBodyIndex :type Integer))
  ;[1 1 1] BoxTrigger
  (set `self.IsOverlap_MainChar` false))

(event `Key|W`
  (params (Key :type "Key Structure"))
  (bind _box (`self.Box`))
  ;[1 1 1] Change Trigger Box Transform
  (:`Pressed`
    (if (`self.PressAbsorb`)
      (`self.ChangeTriggerBoxTransAbsrob` _box (56.0 0.0 0.0) (struct :`Yaw` 90.0))
      (elif (`self.PressSkill`)
        (`self.ChangeTriggerBoxTransSkill` _box (56.0 0.0 0.0) (struct :`Yaw` 90.0))))))

(event `Key|S`
  (params (Key :type "Key Structure"))
  (bind _box (`self.Box`))
  ;[1 1 1] Change Trigger Box Transform
  (:`Pressed`
    (if (`self.PressAbsorb`)
      (`self.ChangeTriggerBoxTransAbsrob` _box (-56.0 0.0 0.0) (struct :`Yaw` 90.0))
      (elif (`self.PressSkill`)
        (`self.ChangeTriggerBoxTransSkill` _box (-56.0 0.0 0.0) (struct :`Yaw` 90.0))))))

(event `ReMatter`
  ;[1 1 1] Change to Normal
  (set `self.SkillIndex` 0)
  (`PrimitiveComponent.SetMaterial` (`self.Sphere`) 0 "/Game/Materials/Material/Trail_Test.Trail_Test")
  (`PrimitiveComponent.SetMaterial` (`self.Plane`) 0 "/Game/Materials/Material/Trail_Test.Trail_Test"))

(event `UseFire`
  (bind _itemre (`self.ItemRe`))
  ;[1 1 1] FireSkill
  (if (`self.IsOverlap_MainChar`)
    (if (`KismetSystemLibrary.DoesImplementInterface` _itemre "/Game/Blueprint/BPI_MainBallSkill.BPI_MainBallSkill_C")
      (message `/Game/Blueprint/BPI_MainBallSkill.Fire` _itemre))))

(event `Key|D`
  (params (Key :type "Key Structure"))
  (bind _box (`self.Box`))
  ;[1 1 1] Change Trigger Box Transform
  (:`Pressed`
    (if (`self.PressAbsorb`)
      (`self.ChangeTriggerBoxTransAbsrob` _box (0.0 56.0 0.0))
      (elif (`self.PressSkill`)
        (`self.ChangeTriggerBoxTransSkill` _box (0.0 56.0 0.0))))))

(event `UseWater`
  (bind _itemre (`self.ItemRe`))
  ;[1 1 1] WaterSkill
  (if (`self.IsOverlap_MainChar`)
    (if (`KismetSystemLibrary.DoesImplementInterface` _itemre "/Game/Blueprint/BPI_MainBallSkill.BPI_MainBallSkill_C")
      (message `/Game/Blueprint/BPI_MainBallSkill.Water` _itemre))))

(event `Key|A`
  (params (Key :type "Key Structure"))
  (bind _box (`self.Box`))
  ;[1 1 1] Change Trigger Box Transform
  (:`Pressed`
    (if (`self.PressAbsorb`)
      (`self.ChangeTriggerBoxTransAbsrob` _box (0.0 -80.0 0.0))
      (elif (`self.PressSkill`)
        (`self.ChangeTriggerBoxTransSkill` _box (0.0 -80.0 0.0) (struct :`Yaw` 180.0))))))

(event `UseIce`
  (bind _itemre (`self.ItemRe`))
  ;[1 1 1] Ice Skill
  (if (`self.IsOverlap_MainChar`)
    (if (`KismetSystemLibrary.DoesImplementInterface` _itemre "/Game/Blueprint/BPI_MainBallSkill.BPI_MainBallSkill_C")
      (message `/Game/Blueprint/BPI_MainBallSkill.Ice` _itemre))))

(fn `ChangeTriggerBoxTransAbsrob`
  (params (TriggerBox :type "SceneComponent Object Reference") (NewLocation :type "Vector Structure") (NewRotation :type "Rotator Structure")))

(fn `ChangeTriggerBoxTransSkill`
  (params (TriggerBox :type "SceneComponent Object Reference") (NewLocation :type "Vector Structure") (NewRotation :type "Rotator Structure"))
  (`SceneComponent.K2_SetRelativeRotation` TriggerBox NewRotation false false)
  (`SceneComponent.K2_SetRelativeLocation` TriggerBox NewLocation false false)
  (`SceneComponent.SetVisibility` (`self.PlaneSkill`) true false))

(fn `ResetMatter`)

(fn `ResetTriggerBoxTrans`
  (params (TriggerBox :type "SceneComponent Object Reference") (NewLocation :type "Vector Structure") (NewRotation :type "Rotator Structure"))
  (`SceneComponent.K2_SetRelativeRotation` TriggerBox NewRotation false false)
  (`SceneComponent.K2_SetRelativeLocation` TriggerBox NewLocation false false)
  (`SceneComponent.SetVisibility` (`self.Plane`) true false))

(fn `UserConstructionScript`)