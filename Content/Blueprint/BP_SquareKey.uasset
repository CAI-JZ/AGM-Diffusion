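; BP_SquareKey is a key actor with a cube and sphere that can be highlighted and given a Fire, Water or Ice element.
; Hightlight swaps the cube's material and registers the actor as HighLightActor in BP_Instance, while StopHighLight restores only the moss material.
; Each element event nudges the sphere upward, applies that element's material and sets the matching power flag on the game instance.
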(event `/Game/Blueprint/BPI_MainBallSkill.Hightlight`
  ;[1 1 1] HightLight
  (`PrimitiveComponent.SetMaterial` (`self.Cube`) 0 "/Game/Materials/Highlight_Inst.Highlight_Inst")
  (bind _asbp_instance (cast `/Game/Blueprint/BP_Instance` (`GameplayStatics.GetGameInstance`)))
  (set `/Game/Blueprint/BP_Instance.HighLightActor` self _asbp_instance))

(event `/Game/Blueprint/BPI_MainBallSkill.StopHighLight`
  ;[1 1 1] HightLight
  (`PrimitiveComponent.SetMaterial` (`self.Cube`) 0 "/Game/StarterContent/Materials/M_Ground_Moss.M_Ground_Moss"))

(event `/Game/Blueprint/BPI_MainBallSkill.Fire`
  (bind _sphere (`self.Sphere`))
  (`SceneComponent.K2_AddLocalOffset` _sphere (0.0 0.0 30.0) false false)
  (`PrimitiveComponent.SetMaterial` _sphere 0 "/Game/Materials/Trail_Fire.Trail_Fire")
  (bind _asbp_instance (cast `/Game/Blueprint/BP_Instance` (`GameplayStatics.GetGameInstance`)))
  (set `/Game/Blueprint/BP_Instance.FirePower?` true _asbp_instance))

(event `/Game/Blueprint/BPI_MainBallSkill.Water`
  (bind _sphere (`self.Sphere`))
  (`SceneComponent.K2_AddLocalOffset` _sphere (0.0 0.0 30.0) false false)
  (`PrimitiveComponent.SetMaterial` _sphere 0 "/Game/StarterContent/Materials/M_Water_Ocean.M_Water_Ocean")
  (bind _asbp_instance (cast `/Game/Blueprint/BP_Instance` (`GameplayStatics.GetGameInstance`)))
  (set `/Game/Blueprint/BP_Instance.WaterPower?` true _asbp_instance))

(event `/Game/Blueprint/BPI_MainBallSkill.Ice`
  (bind _sphere (`self.Sphere`))
  (`SceneComponent.K2_AddLocalOffset` _sphere (0.0 0.0 30.0) false false)
  (`PrimitiveComponent.SetMaterial` _sphere 0 "/Game/Materials/StylizedWaterAndIceMaterials/Materials/M_Ice04.M_Ice04")
  (bind _asbp_instance (cast `/Game/Blueprint/BP_Instance` (`GameplayStatics.GetGameInstance`)))
  (set `/Game/Blueprint/BP_Instance.IcePower?` true _asbp_instance))

(fn `UserConstructionScript`)