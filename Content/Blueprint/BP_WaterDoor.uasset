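; BP_WaterDoor is a highlightable door actor that opens when water power is on.
; Highlight events swap the Cube material between a highlight instance and moss, and highlighting registers the actor as HighLightActor on the BP_Instance game instance.
; Tick polls the game instance's WaterPower flag and, after a short delay, opens the door by hiding the Door mesh and disabling its collision.
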(event `/Game/Blueprint/BPI_MainBallSkill.Hightlight`
  ;[1 1 1] HighLight
  (`PrimitiveComponent.SetMaterial` (`self.Cube`) 0 "/Game/Materials/Highlight_Inst.Highlight_Inst")
  (bind _asbp_instance (cast `/Game/Blueprint/BP_Instance` (`GameplayStatics.GetGameInstance`)))
  (set `/Game/Blueprint/BP_Instance.HighLightActor` self _asbp_instance))

(event `/Game/Blueprint/BPI_MainBallSkill.StopHighLight`
  ;[1 1 1] HighLight
  (`PrimitiveComponent.SetMaterial` (`self.Cube`) 0 "/Game/StarterContent/Materials/M_Ground_Moss.M_Ground_Moss"))

(event `self.ReceiveTick`
  (params (DeltaSeconds :type "Float (single-precision)"))
  (bind _door (`self.Door`))
  ;[1 1 1] OpenDoor
  (bind _asbp_instance (cast `/Game/Blueprint/BP_Instance` (`GameplayStatics.GetGameInstance`)))
  (if (`/Game/Blueprint/BP_Instance.WaterPower?` _asbp_instance)
    (`KismetSystemLibrary.Delay` 0.2)
    (`SceneComponent.SetVisibility` _door false false)
    (`PrimitiveComponent.SetCollisionEnabled` _door "NoCollision")))

(fn `UserConstructionScript`)