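; BP_Ice is an ice object that the player ball can absorb or that fire turns into water.
; Absorbing plays a timeline in reverse to drive scale and Niagara parameters, then destroys the mesh and gives PB_MainBall the ice skill, material and light color.
; Fire rescales and destroys it, spawns BP_Water below and resets the ball's matter.
; Highlight events swap materials, registering the actor with BP_Instance when highlighted.
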(event `/Game/Blueprint/BPI_MainBallSkill.AbsorbProcess`
  ;[1 1 1] Comment
  ;;[1 1 1] Comment
  (bind (_direction _newtrack_0) (`Timeline|Timeline_0` :!via `ReverseFromEnd`)
    (:`Update`
      (`SceneComponent.SetWorldScale3D` (`self.Base`) (`KismetMathLibrary.Conv_DoubleToVector` _newtrack_0))
      (`self.NewMacro_0` (`self.Niagara`) _newtrack_0))
    (:`Finished`
      ;;[1 1 1] Comment
      (`self.IceDisappear`)
      (bind _aspb_main_ball (cast `/Game/Blueprint/PB_MainBall` (`GameplayStatics.GetPlayerPawn` 0)))
      (set `/Game/Blueprint/PB_MainBall.SkillIndex` 3 _aspb_main_ball)
      (`PrimitiveComponent.SetMaterial` (`/Game/Blueprint/PB_MainBall.Sphere` _aspb_main_ball) 0 "/Game/Materials/M_AbsorbIce.M_AbsorbIce")
      (`LightComponent.SetLightColor` (`/Game/Blueprint/PB_MainBall.PointLight` _aspb_main_ball) (struct :`R` 0.528941 :`G` 0.858413 :`B` 1.0 :`A` 1.0) true)
      (`KismetSystemLibrary.Delay` 0.2)
      (`self.NewMacro_0` (`self.Niagara`)))))

(event `/Game/Blueprint/BPI_MainBallSkill.Fire`
  ;[1 1 1] Comment
  (bind (_direction _newtrack_0) (`Timeline|Timeline_1` :!via `ReverseFromEnd`)
    (:`Update`
      (`SceneComponent.SetWorldScale3D` (`self.Base`) (`KismetMathLibrary.Conv_DoubleToVector` _newtrack_0)))
    (:`Finished`
      (`self.IceDisappear`)
      (`|SpawnActorFromClass` "/Game/Blueprint/BP_Water.BP_Water_C" (`KismetMathLibrary.MakeTransform` (`KismetMathLibrary.MakeVector` (.x (.location (`SceneComponent.K2_GetComponentToWorld` (`self.Root`)))) (.y (.location (`SceneComponent.K2_GetComponentToWorld` (`self.Root`)))) (- (.z (.location (`SceneComponent.K2_GetComponentToWorld` (`self.Root`)))) 100.0)) (.rotation (`SceneComponent.K2_GetComponentToWorld` (`self.Root`))) (.scale (`SceneComponent.K2_GetComponentToWorld` (`self.Root`)))) "AlwaysSpawn" "OverrideRootScale" null null)
      (bind _aspb_main_ball (cast `/Game/Blueprint/PB_MainBall` (`GameplayStatics.GetPlayerPawn` 0)))
      (`/Game/Blueprint/PB_MainBall.ResetMatter` _aspb_main_ball))))

(event `/Game/Blueprint/BPI_MainBallSkill.Hightlight`
  ;[1 1 1] HighLight
  (`PrimitiveComponent.SetMaterial` (`self.Base`) 0 "/Game/Materials/Highlight_Inst.Highlight_Inst")
  (bind _asbp_instance (cast `/Game/Blueprint/BP_Instance` (`GameplayStatics.GetGameInstance`)))
  (set `/Game/Blueprint/BP_Instance.HighLightActor` self _asbp_instance))

(event `/Game/Blueprint/BPI_MainBallSkill.StopHighLight`
  (bind _base (`self.Base`))
  ;[1 1 1] StopHighlight
  (if (`KismetSystemLibrary.IsValid` _base)
    (`PrimitiveComponent.SetMaterial` _base 0 "/Game/Materials/M_ICE_Inst.M_ICE_Inst")))

(fn `IceDisappear`
  (`ActorComponent.K2_DestroyComponent` (`self.Base`)))

(fn `UserConstructionScript`)