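; BP_Water is a water object that the player ball can absorb as an element or turn to ice, with highlighting registered in BP_Instance.
; Absorbing reverses a timeline that scales the water and Niagara effect, then gives PB_MainBall the water skill, material and light before destroying the actor.
; Ice swaps it for BP_Ice and resets the ball's matter, while Fire and Water only play a sound.
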(event `self.ReceiveBeginPlay`
  (set `self.HasWater` true))

(event `/Game/Blueprint/BPI_MainBallSkill.AbsorbProcess`
  ;[1 1 1] Comment
  ;;[1 1 1] Comment
  (bind (_direction _newtrack_0) (`Timeline|Timeline_0` :!via `ReverseFromEnd`)
    (:`Update`
      (`SceneComponent.SetRelativeScale3D` (`self.Water_0`) (`KismetMathLibrary.Conv_DoubleToVector` _newtrack_0))
      (`self.AbsorbNiagaraSet` (`self.Niagara`) _newtrack_0))
    (:`Finished`
      ;;[1 1 1] Comment
      (`self.WaterDisappear`)
      (bind _aspb_main_ball (cast `/Game/Blueprint/PB_MainBall` (`GameplayStatics.GetPlayerPawn` 0)))
      (set `/Game/Blueprint/PB_MainBall.SkillIndex` 2 _aspb_main_ball)
      (`PrimitiveComponent.SetMaterial` (`/Game/Blueprint/PB_MainBall.Sphere` _aspb_main_ball) 0 "/Game/Materials/M_AbsorbWater.M_AbsorbWater")
      (bind _pointlight (`/Game/Blueprint/PB_MainBall.PointLight` _aspb_main_ball))
      (`LightComponent.SetLightColor` _pointlight (struct :`R` 0.3675 :`G` 0.864418 :`B` 0.909722 :`A` 1.0) true)
      (`LightComponent.SetIntensity` _pointlight 4000.0)
      (`KismetSystemLibrary.Delay` 0.2)
      (`self.AbsorbNiagaraSet` (`self.Niagara`))
      (`self.K2_DestroyActor`))))

(event `/Game/Blueprint/BPI_MainBallSkill.Fire`
  (`GameplayStatics.PlaySound2D` "/Game/One_Hundred_Game_SFX/Cues/CUE_UI_Game_Pop_3_Cue.CUE_UI_Game_Pop_3_Cue" 1.0 1.0 0.0 null null))

(event `/Game/Blueprint/BPI_MainBallSkill.Ice`
  ;[1 1 1] Comment
  (`|SpawnActorFromClass` "/Game/Blueprint/BP_Ice.BP_Ice_C" (`SceneComponent.K2_GetComponentToWorld` (`self.Root`)) "Undefined" "OverrideRootScale" null null)
  (`self.K2_DestroyActor`)
  (bind _aspb_main_ball (cast `/Game/Blueprint/PB_MainBall` (`GameplayStatics.GetPlayerPawn` 0)))
  (`/Game/Blueprint/PB_MainBall.ResetMatter` _aspb_main_ball)
  (`GameplayStatics.PlaySound2D` "/Game/One_Hundred_Game_SFX/Cues/CUE_UI_Bright_Confirmation_Button_5_Cue.CUE_UI_Bright_Confirmation_Button_5_Cue" 1.0 1.0 0.0 null null))

(event `/Game/Blueprint/BPI_MainBallSkill.Water`
  (`GameplayStatics.PlaySound2D` "/Game/One_Hundred_Game_SFX/Cues/CUE_UI_Game_Pop_3_Cue.CUE_UI_Game_Pop_3_Cue" 1.0 1.0 0.0 null null))

(event `/Game/Blueprint/BPI_MainBallSkill.Hightlight`
  ;[1 1 1] HighLight
  (if (`self.HasWater`)
    (`PrimitiveComponent.SetMaterial` (`self.Water_0`) 0 "/Game/Materials/M_Highlight_Inst_Water.M_Highlight_Inst_Water")
    (bind _asbp_instance (cast `/Game/Blueprint/BP_Instance` (`GameplayStatics.GetGameInstance`)))
    (set `/Game/Blueprint/BP_Instance.HighLightActor` self _asbp_instance)
    (else
      (`PrimitiveComponent.SetMaterial` (`self.Water_1`) 0 "/Game/Materials/M_Highlight_Inst_Normal.M_Highlight_Inst_Normal")
      (bind _asbp_instance_2 (cast `/Game/Blueprint/BP_Instance` (`GameplayStatics.GetGameInstance`)))
      (set `/Game/Blueprint/BP_Instance.HighLightActor` self _asbp_instance_2))))

(event `/Game/Blueprint/BPI_MainBallSkill.StopHighLight`
  ;[1 1 1] StopHighLight
  (if (`self.HasWater`)
    (`PrimitiveComponent.SetMaterial` (`self.Water_0`) 0 "/Game/StarterContent/Materials/M_Water_Ocean.M_Water_Ocean")
    (else
      (`PrimitiveComponent.SetMaterial` (`self.Water_1`) 0 "/Game/StylizedRuinsProps/Materials/M_Stone02.M_Stone02"))))

(fn `UserConstructionScript`)

(fn `WaterDisappear`
  (`GameplayStatics.PlaySound2D` "/Game/One_Hundred_Game_SFX/Cues/CUE_UI_Bright_Confirmation_Button_1_Cue.CUE_UI_Bright_Confirmation_Button_1_Cue" 1.0 1.0 0.0 null null))